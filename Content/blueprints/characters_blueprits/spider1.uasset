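; Spider enemy character that chases the player, attacks at close range and dies when its health runs out.
; An AIMoveTo loop re-targets the player while Tick checks distance and plays the attack montage, pausing movement and applying damage on completion.
; AnyDamage reduces health; on death it stops movement, increments the soldier's kill count, destroys itself after a delay and registers the death with the gamemode.
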(event EventBeginPlay
  ;[0.04383 0.1371 0.15 0.5] movement
  (if (not (Variables|Default|GetSpider%20Death)) :!label _label
    (AI|AIMoveTo self "0, 0, 0" (Game|GetPlayerCharacter 0) 5.0 (Variables|Default|GetSpider%20Death)
      (:OnSuccess
        _)
      (:OnFail
        _))
    (Utilities|FlowControl|Delay 0.2)
    (goto _label)))

(event Game|Damage|EventAnyDamage
  (params (Damage :type Float%20%28single-precision%29) (DamageType :type Damage%20Type%20Object%20Reference) (InstigatedBy :type Controller%20Object%20Reference) (DamageCauser :type Actor%20Object%20Reference))
  ;[0.15 0.15 0.15 0.5] r.i.p. mechanics
  (bind _isspiderdead (CallFunction|CheckSpiderDeath Damage))
  (if _isspiderdead
    (Components|Activation|Deactivate (Variables|Character|GetCharacterMovement))
    (Development|PrintString "Hello")
    (CallFunction|IncrementKills)
    ;[0.15 0.03729 0.06228 0.5] spider attack
    (Components|Movement|StopMovementImmediately (Variables|Character|GetCharacterMovement))
    (Utilities|FlowControl|Delay 2.0)
    (Actor|DestroyActor)
    (bind _asgamemode (Utilities|Casting|CastTogamemode (Game|GetGameMode)))
    (Default|RegisterSpiderDeath _asgamemode self)))

(event EventTick
  (params (DeltaSeconds :type Float%20%28single-precision%29))
  ;[0.15 0.03729 0.06228 0.5] spider attack
  (if (not (Variables|Default|GetSpider%20Death))
    (if (and (CallFunction|IsAttackRange) (not (CallFunction|IsAttacking)))
      (Components|Activation|Deactivate (Variables|Character|GetCharacterMovement))
      (Development|PrintString "jpdl")
      (Animation|Montage|PlayMontage (Variables|Character|GetMesh) "/Game/Characters/Enemy_Great_Spider/Animations/Spider_Attack_02.Spider_Attack_02" 2.0
        (:OnCompleted
          (Components|Activation|Activate (Variables|Character|GetCharacterMovement) false)
          (Game|Damage|ApplyDamage (Game|GetPlayerCharacter 0) 15.0 0 0))))))

(event Input|KeyboardEvents|SpaceBar
  (params (Key :type Key%20Structure :default "None"))
  (:Pressed
    (Components|Activation|Deactivate (Variables|Character|GetCharacterMovement))
    (Animation|Montage|PlayMontage (Variables|Character|GetMesh) 0 2.0
      (:OnCompleted
        (Components|Activation|Activate (Variables|Character|GetCharacterMovement) false)))))

(fn ConstructionScript)

(fn IsAttackRange
  (bind _asbp_soldier (Utilities|Casting|CastToBP_Soldier (Game|Player|GetPlayerPawn 0)))
  (return (< (Transformation|GetDistanceTo _asbp_soldier) 1e+02)))

(fn IsAttacking
  (return (Animation|Montage|MontageIsPlaying (Components|SkeletalMesh|GetAnimInstance (Variables|Character|GetMesh)) "/Game/Characters/Enemy_Great_Spider/Animations/Spider_Attack_02.Spider_Attack_02")))

(fn CheckSpiderDeath
  (params (Damage :type Float%20%28double-precision%29))
  (bind _output_get (Variables|Default|SetSpider%20Health (Math|Float|Clamp(Float) (- (Variables|Default|GetSpider%20Health) Damage) 0.0 1e+02)))
  (if (== _output_get 0.0)
    (bind _output_get_2 (Variables|Default|SetSpider%20Death true))
    (return _output_get_2)))

(fn IncrementKills
  (bind _asbp_soldier (Utilities|Casting|CastToBP_Soldier (Game|GetPlayerCharacter 0)))
  (Variables|Default|SetAs%20BP%20Soldier _asbp_soldier)
  (bind _result (Math|Integer|IncrementInt (Variables|/Game/blueprints/characters_blueprits/BP_Soldier.BP_Soldier_C|GetKills (Variables|Default|GetAs%20BP%20Soldier)))
    (:%20%20
      (Variables|/Game/blueprints/characters_blueprits/BP_Soldier.BP_Soldier_C|SetKills (Variables|Default|GetAs%20BP%20Soldier) _result))))