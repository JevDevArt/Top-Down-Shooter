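; Game mode that runs escalating waves of enemy spiders, starting shortly after play begins.
; Each wave scales the previous spider count by a difficulty multiplier, then a looping named timer spawns spiders at random TargetPoints until the quota runs out.
; From the third wave onward, spawned spiders are larger, with overridden health and attack distance.
; RegisterSpiderDeath removes spiders from the tracked array, starting the next wave once none remain to spawn or kill.
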(event Custom|SpawnSpider
  (bind _returnvalue (CallFunction|EnemySpawn))
  (Utilities|Array|Add (Variables|Default|Getspiders) _returnvalue)
  (bind _result (Math|Integer|DecrementInt (Variables|Default|Getspider%20Remaining))
    (:%20%20
      (bind _output_get (Variables|Default|Setspider%20Remaining _result))
      (if (== _output_get 0)
        (Utilities|Time|ClearTimerbyFunctionName 0 "SpawnSpider")))))

(event Custom|EndWave
  (CallFunction|StartNewWave))

(event EventBeginPlay
  (Utilities|FlowControl|Delay 2.0)
  (CallFunction|StartNewWave))

(event EventTick
  (params (DeltaSeconds :type Float%20%28single-precision%29)))

(fn ConstructionScript)

(fn EnemySpawn
  (bind _outactors (Actor|GetAllActorsOfClass "/Script/Engine.TargetPoint"))
  (bind _returnvalue (Game|SpawnActorfromClass "/Game/blueprints/characters_blueprits/spider1.spider1_C" (Transformation|GetActorTransform (Utilities|Array|Get(acopy) _outactors (Math|Random|RandomIntegerinRange 0 (Utilities|Array|LastIndex _outactors)))) "Undefined" "MultiplyWithRoot" 0 0))
  (if (>= (Variables|Default|Getwave%20number) 3)
    (CallFunction|ChangeSpidersParams _returnvalue))
  (return _returnvalue))

(fn RegisterSpiderDeath
  (params (Item :type Spider%201%20Object%20Reference%20%28by%20ref%29))
  (Utilities|Array|RemoveItem (Variables|Default|Getspiders) Item)
  (if (and (== (Variables|Default|Getspider%20Remaining) 0) (== (Utilities|Array|Length (Variables|Default|Getspiders)) 0))
    (CallFunction|EndWave)))

(fn StartNewWave
  (Math|Integer|IncrementInt (Variables|Default|Getwave%20number)
    (:%20%20
      (CallFunction|DiffWave)
      (Utilities|Time|SetTimerbyFunctionName 0 "SpawnSpider" 2.0 true))))

(fn DiffWave
  (bind _output_get (Variables|Default|Setspider%20Remaining (Math|Float|Round (* (Variables|Default|GetSpiderLastLevel) (Variables|Default|GetDiffLevel)))))
  (Variables|Default|SetSpiderLastLevel _output_get))

(fn ChangeSpidersParams
  (params (SpawnedMoreHPSpider :type Spider%201%20Object%20Reference))
  (bind _output_get (Variables|Default|SetSpawnedMoreHPSpider SpawnedMoreHPSpider))
  (Variables|/Game/blueprints/characters_blueprits/spider1.spider1_C|SetSpider%20Health _output_get 2e+02)
  (Transformation|SetActorScale3D _output_get (* (Transformation|GetActorScale3D _output_get) 2.0))
  (Variables|/Game/blueprints/characters_blueprits/spider1.spider1_C|SetAttack%20Disctance _output_get 2e+02))